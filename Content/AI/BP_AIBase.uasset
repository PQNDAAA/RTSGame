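; BP_AIBase is an AI pawn that moves toward the location of a Base actor in the level.
; Every Tick it looks up that actor with GetActorOfClass and reissues AIMoveTo to its current location with a small acceptance radius.
; The construction script gives the Cube mesh a dynamic material instance with a random Color, so instances vary in tint.
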(event EventTick
  (params (DeltaSeconds :type Float%20%28single-precision%29))
  (bind _returnvalue (Actor|GetActorOfClass (Variables|Default|Getbase)))
  (AI|AIMoveTo self (Transformation|GetActorLocation _returnvalue) 0 2e+01 false))

(fn ConstructionScript
  (bind _returnvalue (Rendering|Material|CreateDynamicMaterialInstance (Variables|Default|GetCube) 0 0 "None" :!class /Script/Engine.PrimitiveComponent))
  (Rendering|Material|SetVectorParameterValue _returnvalue "Color" (Math|Color|MakeColor (Math|Random|RandomFloat) (Math|Random|RandomFloat) (Math|Random|RandomFloat)) :!class /Script/Engine.MaterialInstanceDynamic))